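; Collectable package world object that plays a hop-and-spin animation when interacted with, and sets its ID to "Package" at construction.
; Interact chains two timed MoveComponentTo moves on ScaleScene, lifting it and returning it while changing yaw.
; IsInteractable is off during the animation, then NewRotation is updated for the next spin.
; Interact does not call the parent implementation; a note flags this as pending.
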(event EventInteract
  (params (Sender :type Actor%20Object%20Reference))
  (Variables|Default|SetIsInteractable false)
  (Components|MoveComponentTo (Variables|Default|GetScaleScene) "0.000000,0.000000,100.000000" (Math|Rotator|MakeRotator 0.0 0.0 (+ (Variables|Default|GetRotationAnimationStrength) (Variables|Default|GetNewRotation))) false false 0.5 false)
  (Components|MoveComponentTo (Variables|Default|GetScaleScene) "0, 0, 0" (Math|Rotator|MakeRotator 0.0 0.0 (* (+ (Variables|Default|GetRotationAnimationStrength) (Variables|Default|GetNewRotation)) 2.0)) false false 0.5 false)
  (Variables|Default|SetIsInteractable true)
  (Variables|Default|SetNewRotation (+ (Variables|Default|GetRotationAnimationStrength) 1.8e+02)))

(fn ConstructionScript
  (|CallParentFunction)
  (Variables|Default|SetID "Package"))
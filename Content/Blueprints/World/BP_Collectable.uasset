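; BP_Collectable is a world item the player can pick up and carry, one at a time.
; On interact, if the player's hands are empty, it becomes the HeldCollectable, disables collision, waits a tick, snaps to the player's CollectablePivot, stops casting shadows and calls its collected dispatcher.
; PlaceCollectable restores shadow and collision, while separate functions set and report whether it is interactable.
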(event Custom|PlaceCollectable
  (Rendering|SetCastShadow (Variables|Default|GetMesh) true)
  (Collision|SetCollisionEnabled (Variables|Default|GetMesh) "QueryAndPhysics"))

(event EventSetInteractStatus
  (params (IsInteractable :type Boolean))
  (Variables|Default|SetIsInteractable IsInteractable))

(event EventInteract
  (params (Sender :type Actor%20Object%20Reference))
  (bind _asbp_player (Utilities|Casting|CastToBP_Player Sender))
  (Variables|/Game/Blueprints/Core/BP_Player.BP_Player_C|GetHeldCollectable _asbp_player
    (:then)
    (:else
      (Variables|/Game/Blueprints/Core/BP_Player.BP_Player_C|SetHeldCollectable _asbp_player self)
      (Collision|SetCollisionEnabled (Variables|Default|GetMesh) "NoCollision")
      (Utilities|FlowControl|DelayUntilNextTick)
      (Transformation|AttachComponentToComponent (Variables|/Game/Blueprints/Core/BP_Player.BP_Player_C|GetCollectablePivot _asbp_player) "None" "SnapToTarget" "SnapToTarget" "SnapToTarget" true)
      (Rendering|SetCastShadow (Variables|Default|GetMesh) false)
      (Default|CallOnCollectedDispatcher))))

(fn ConstructionScript)

(fn ReturnInteractStatus
  (return (Variables|Default|GetIsInteractable)))
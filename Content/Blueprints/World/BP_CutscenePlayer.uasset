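; BP_CutscenePlayer plays a level sequence when it receives a solved React event, then relays the reaction to a target actor.
; During playback it pushes an activatable widget onto the main UI stack and increments the player's CantMove counter, undoing both when the sequence finishes.
; The target's ReactMessage fires after ReactDelay, or immediately with false when unsolved.
; An optional play-once gate makes later solves skip the cutscene and notify the target directly.
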(event Custom|OnCutsceneEnded
  (Class|CommonActivatableWidgetContainerBase|RemoveWidget (Utilities|ReturnMainStack (Game|GetPlayerController 0)) (Variables|Default|GetActiveWidget))
  (bind _playerref (Variables|Default|GetPlayerRef)
    (:then
      (Math|Integer|DecrementInt (Variables|/Game/Blueprints/Core/BP_Player.BP_Player_C|GetCantMove _playerref)))
    (:else)))

(event EventReact
  (params (Solved :type Boolean))
  (bind _cutscenetoplay (Variables|Default|GetCutsceneToPlay))
  (bind _sequenceplayer (Variables|/Script/LevelSequence.LevelSequenceActor|GetSequencePlayer _cutscenetoplay))
  (if Solved
    (bind _returnvalue (Class|CommonActivatableWidgetContainerBase|AddWidget (Utilities|ReturnMainStack (Game|GetPlayerController 0)) (Variables|Default|GetActivatableWidget)))
    (Variables|Default|SetActiveWidget _returnvalue)
    (Variables|Default|GetPlayOnce
      (:then
        (Utilities|DoOncewithAfter
          (:Completed
            (Utilities|FlowControl|Sequence :!label _label
              (:then_0
                (Variables|Default|GetPlayerRef
                  (:then
                    _)
                  (:else
                    (bind _returnvalue_2 (Actor|GetActorOfClass "/Game/Blueprints/Core/BP_Player.BP_Player_C"))
                    (Variables|Default|SetPlayerRef _returnvalue_2)))
                (Math|Integer|IncrementInt (Variables|/Game/Blueprints/Core/BP_Player.BP_Player_C|GetCantMove (Variables|Default|GetPlayerRef))
                  (:%20%20
                    (Sequencer|Player|Play _sequenceplayer :!class /Script/MovieScene.MovieSceneSequencePlayer)
                    (Class|CommonActivatableWidgetContainerBase|AddWidget (Utilities|ReturnMainStack (Game|GetPlayerController 0)) (Variables|Default|GetActivatableWidget))
                    (EventDispatchers|BindEventtoOnFinished _sequenceplayer (delegate Custom|OnCutsceneEnded)))))
              (:then_1
                (Utilities|FlowControl|Delay (Variables|Default|GetReactDelay))
                (Class|BPIReact|React(Message) (Variables|Default|GetActorToReact) true))))
          (:After
            (Class|CommonActivatableWidgetContainerBase|RemoveWidget (Utilities|ReturnMainStack (Game|GetPlayerController 0)) (Variables|Default|GetActiveWidget))
            (Class|BPIReact|React(Message) (Variables|Default|GetActorToReact) true))))
      (:else
        (goto _label)))
    (else
      (Class|BPIReact|React(Message) (Variables|Default|GetActorToReact) false))))

(fn ConstructionScript)
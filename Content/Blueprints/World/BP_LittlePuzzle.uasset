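; BP_LittlePuzzle is a possessable dial puzzle with a random solution index, which it passes to a hint actor on BeginPlay.
; Interacting smoothly possesses it and shows a widget, and pressing interact again returns control to the player.
; Left/right input cycles the mesh through preset rotations, messaging ActorToReact as the solved state changes.
; React toggles its interactability and swaps copper materials to show it.
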(event Custom|Down)

(event Custom|Left
  (Variables|Default|SetCurrentPositionIndex (Math|Integer|SelectInt (Utilities|Array|LastIndex (Variables|Default|GetRotationPoints)) (- (Variables|Default|GetCurrentPositionIndex) 1) (< (- (Variables|Default|GetCurrentPositionIndex) 1) 0)))
  (Transformation|SetRelativeRotation (Variables|Default|GetR1Mesh) (Utilities|Array|Get(acopy) (Variables|Default|GetRotationPoints) (Variables|Default|GetCurrentPositionIndex)) true false) ; Smooth Movement = Sweep
  (if (== (Variables|Default|GetCurrentPositionIndex) (Variables|Default|GetSolvedPositionIndex))
    (Variables|Default|SetSolved true)
    (Class|BPIReact|React(Message) (Variables|Default|GetActorToReact) true)
    (goto _label Reset)
    (else
      (Variables|Default|GetSolved
        (:then
          (Variables|Default|SetSolved false)
          (Utilities|FlowControl|DoOnce true :!label _label
            (:Completed
              (Class|BPIReact|React(Message) (Variables|Default|GetActorToReact) false))))
        (:else)))))

(event Custom|Right
  (Variables|Default|SetCurrentPositionIndex (Math|Integer|SelectInt 0 (+ (Variables|Default|GetCurrentPositionIndex) 1) (> (+ (Variables|Default|GetCurrentPositionIndex) 1) (Utilities|Array|LastIndex (Variables|Default|GetRotationPoints)))))
  (Transformation|SetRelativeRotation (Variables|Default|GetR1Mesh) (Utilities|Array|Get(acopy) (Variables|Default|GetRotationPoints) (Variables|Default|GetCurrentPositionIndex)) true false) ; Smooth Movement = Sweep
  (if (== (Variables|Default|GetCurrentPositionIndex) (Variables|Default|GetSolvedPositionIndex))
    (Variables|Default|SetSolved true)
    (Class|BPIReact|React(Message) (Variables|Default|GetActorToReact) true)
    (goto _label Reset)
    (else
      (Variables|Default|GetSolved
        (:then
          (Variables|Default|SetSolved false)
          (Utilities|FlowControl|DoOnce true :!label _label
            (:Completed
              (Class|BPIReact|React(Message) (Variables|Default|GetActorToReact) false))))
        (:else)))))

(event Custom|Up)

(event Input|EnhancedActionEvents|EnhancedInputActionIA_Interact
  (params (ActionValue :type Boolean) (ElapsedSeconds :type Float%20%28double-precision%29) (TriggeredSeconds :type Float%20%28double-precision%29) (InputAction :type Input%20Action%20Object%20Reference :default "/Game/Inputs/IA_Interact.IA_Interact"))
  (:Started
    (Class|CommonActivatableWidgetContainerBase|RemoveWidget (Utilities|ReturnMainStack (Game|GetPlayerController 0)) (Variables|Default|GetActiveWidget))
    (Utilities|FlowControl|DoOnce false :!label _label
      (:Completed
        (Utilities|SmoothPossess (Game|GetPlayerController 0) (Variables|Default|GetPlayerRef) 0.5)
        (Pawn|SetControlRotation (Game|GetPlayerController 0) (Variables|Default|GetControlRotation))
        (Math|Integer|DecrementInt (Variables|/Game/Blueprints/Core/BP_Player.BP_Player_C|GetCantMove (Variables|Default|GetPlayerRef))
          (:%20%20
            (goto _label Reset)))))))

(event Input|EnhancedActionEvents|EnhancedInputActionIA_Move
  (params (ActionValue :type Vector%202D%20Structure) (ElapsedSeconds :type Float%20%28double-precision%29) (TriggeredSeconds :type Float%20%28double-precision%29) (InputAction :type Input%20Action%20Object%20Reference :default "/Game/Inputs/IA_Move.IA_Move"))
  (bind (_x _y) (Math|Vector2D|BreakVector2D ActionValue))
  (:Started
    (if (> (Math|Float|Absolute(Float) _x) (Math|Float|Absolute(Float) _y)) ; True = left/right\nFalse = up/down
      (if (> _x 0.0)
        (CallFunction|Right)
        (else
          (CallFunction|Left)))
      (elif (> _y 0.0)
        (CallFunction|Up)
        (else
          (CallFunction|Down))))))

(event EventBeginPlay
  (Variables|Default|SetSolvedPositionIndex (Math|Random|RandomInteger 4))
  (Class|BPIFinalCode|GetCodeNumber(Message) (Variables|Default|GetHintRef) (Utilities|Array|MakeArray (Variables|Default|GetSolvedPositionIndex))))

(event EventReact
  (params (Solved :type Boolean))
  (bind _r1mesh (Variables|Default|GetR1Mesh))
  (bind _r1mesh_2 (Variables|Default|GetR1Mesh))
  (Utilities|FlowControl|FlipFlop
    (:A
      (Rendering|Material|SetMaterial _r1mesh 0 "/Game/Materials/Designer_textures/Copper/MI_Stylized_Copper.MI_Stylized_Copper")
      (Rendering|Material|SetMaterial _r1mesh 1 "/Game/Materials/Designer_textures/Copper/MI_Stylized_Copper.MI_Stylized_Copper")
      (Rendering|Material|SetMaterial (Variables|Default|GetStaticMesh) 0 "/Game/Materials/Designer_textures/Copper/MI_Stylized_OlderCopper.MI_Stylized_OlderCopper")
      (Variables|Default|SetIsInteractable true))
    (:B
      (Rendering|Material|SetMaterial _r1mesh_2 0 "/Game/Materials/Designer_textures/Copper/MI_Stylized_VeryOldCopper.MI_Stylized_VeryOldCopper")
      (Rendering|Material|SetMaterial _r1mesh_2 1 "/Game/Materials/Designer_textures/Copper/MI_Stylized_VeryOldCopper.MI_Stylized_VeryOldCopper")
      (Rendering|Material|SetMaterial (Variables|Default|GetStaticMesh) 0 "/Game/Materials/Designer_textures/Copper/MI_Stylized_VeryOldCopper.MI_Stylized_VeryOldCopper")
      (Variables|Default|SetIsInteractable false))))

(event EventInteract
  (params (Sender :type Actor%20Object%20Reference))
  (bind _asbp_player (Utilities|Casting|CastToBP_Player Sender))
  (bind _output_get (Variables|Default|SetPlayerRef _asbp_player))
  (Math|Integer|IncrementInt (Variables|/Game/Blueprints/Core/BP_Player.BP_Player_C|GetCantMove _output_get)
    (:%20%20
      (Variables|Default|SetControlRotation (Pawn|GetControlRotation (Variables|Default|GetPlayerRef) :!class /Script/Engine.Pawn))
      (Utilities|SmoothPossess (Game|GetPlayerController 0) self 1.0)
      (bind _returnvalue (Class|CommonActivatableWidgetContainerBase|AddWidget (Utilities|ReturnMainStack (Game|GetPlayerController 0)) (Variables|Default|GetActivatableWidget)))
      (Variables|Default|SetActiveWidget _returnvalue))))

(fn ConstructionScript)

(fn ReturnInteractStatus
  (return (Variables|Default|GetIsInteractable)))

(fn ReturnSolvedStatus
  (return (Variables|Default|GetSolved)))
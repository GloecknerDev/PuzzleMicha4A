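; Interactable world object that teleports between its start and target positions, gated by an item ID check on the player.
; On success, a FlipFlop picks TargetTransform or the MoveScene transform saved at BeginPlay and sets the root's relative location, ignoring rotation.
; React triggers the same toggle without the check, and MoveOnce controls whether interaction re-enables afterwards.
; Eased MoveComponentTo logic remains in the graph but never runs.
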(event EventReact
  (params (Solved :type Boolean))
  (bind _isa (Utilities|FlowControl|FlipFlop)
    (:A
      _)
    (:B
      _))
  (Transformation|SetRelativeLocation (Variables|Default|GetDefaultSceneRoot) (.Location (Math|Transform|BreakTransform (Math|Transform|SelectTransform (Variables|Default|GetTargetTransform) (Variables|Default|GetStartTransform) _isa))) false true)
  (Variables|Default|GetMoveOnce
    (:then)
    (:else
      (Variables|Default|SetIsInteractable true))))

(event EventInteract
  (params (Sender :type Actor%20Object%20Reference))
  (Class|KismetSystemLibrary|IsObjectOfSoftClass Sender "/Game/Blueprints/Core/BP_Player.BP_Player_C"
    (:True
      ;[0 0 0 0.5] Check for ID
      (bind _asbp_player (Utilities|Casting|CastToBP_Player Sender))
      (Utilities|CheckforID _asbp_player (Variables|Default|GetNeededID) (Variables|Default|GetDestroyItem)
        (:Success
          (Variables|Default|SetIsInteractable false)
          (bind _isa (Utilities|FlowControl|FlipFlop)
            (:A
              _)
            (:B
              _))
          (Transformation|SetRelativeLocation (Variables|Default|GetDefaultSceneRoot) (.Location (Math|Transform|BreakTransform (Math|Transform|SelectTransform (Variables|Default|GetTargetTransform) (Variables|Default|GetStartTransform) _isa))) false true)
          (Variables|Default|GetMoveOnce
            (:then)
            (:else
              (Variables|Default|SetIsInteractable true))))))
    (:False)))

(event EventBeginPlay
  (Variables|Default|SetStartTransform (Transformation|GetRelativeTransform (Variables|Default|GetMoveScene))))

(fn ConstructionScript)

(fn ReturnInteractStatus
  (return (Variables|Default|GetIsInteractable)))
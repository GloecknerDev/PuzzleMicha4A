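; Possessable three-dial combination puzzle that generates a random solution at BeginPlay and sends it to BP_FinalHint actors.
; Interacting locks player movement, smooth-possesses the puzzle and shows a widget; the interact input restores the player.
; Move input selects a dial vertically and rotates it horizontally, checking all dials against the solution within a tolerance after each turn.
; Solving it notifies ActorToReact, while an incoming React event makes the puzzle interactable.
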(event Custom|Down
  (bind _rotators (Variables|Default|GetRotators))
  (Utilities|IsValid (Variables|Default|GetCurrentRotator)
    (:Is%20Valid
      (Utilities|Array|SetArrayElem (Variables|Default|GetCurrentRotations) (Variables|Default|GetCurrentRotatorIndex) (Variables|/Script/Engine.SceneComponent|GetRelativeRotation (Variables|Default|GetCurrentRotator)))
      (if (< (- (Variables|Default|GetCurrentRotatorIndex) 1) 0)
        (Variables|Default|SetCurrentRotator (Utilities|Array|Get(acopy) _rotators))
        (Variables|Default|SetCurrentRotatorIndex 0)
        (bind _output_get (Variables|Default|SetCurrentRotator (Utilities|Array|Get(acopy) (Variables|Default|GetRotators) (Variables|Default|GetCurrentRotatorIndex))))
        (Transformation|SetRelativeRotation _output_get (Utilities|Array|Get(acopy) (Variables|Default|GetCurrentRotations) (Variables|Default|GetCurrentRotatorIndex)) false false)
        (else
          (Variables|Default|SetCurrentRotator (Utilities|Array|Get(acopy) (Variables|Default|GetRotators) (Math|Integer|Clamp(Integer) (- (Variables|Default|GetCurrentRotatorIndex) 1) 0 (Utilities|Array|LastIndex _rotators))))
          (Variables|Default|SetCurrentRotatorIndex (Math|Integer|Clamp(Integer) (- (Variables|Default|GetCurrentRotatorIndex) 1) 0 (Utilities|Array|LastIndex _rotators)))
          (bind _output_get_2 (Variables|Default|SetCurrentRotator (Utilities|Array|Get(acopy) (Variables|Default|GetRotators) (Variables|Default|GetCurrentRotatorIndex))))
          (Transformation|SetRelativeRotation _output_get_2 (Utilities|Array|Get(acopy) (Variables|Default|GetCurrentRotations) (Variables|Default|GetCurrentRotatorIndex)) false false))))))

(event Custom|Left
  (bind _rotationamount (Variables|Default|GetRotationAmount))
  (bind _currentrotations (Variables|Default|GetCurrentRotations))
  (bind _currentrotatorindex (Variables|Default|GetCurrentRotatorIndex))
  (bind _output (Utilities|Array|Get(acopy) _currentrotations _currentrotatorindex))
  (bind _returnvalue (* _rotationamount -1.0))
  (bind _returnvalue_2 (Math|Rotator|CombineRotators _returnvalue _output))
  (Transformation|SetRelativeRotation (Variables|Default|GetCurrentRotator) _returnvalue_2 false false)
  (Utilities|Array|SetArrayElem (Variables|Default|GetCurrentRotations) (Variables|Default|GetCurrentRotatorIndex) _returnvalue_2)
  (Variables|Default|SetCurrentPositionIndex (Math|Integer|SelectInt (Utilities|Array|LastIndex (Variables|Default|GetRotationPoints)) (- (Variables|Default|GetCurrentPositionIndex) 1) (< (- (Variables|Default|GetCurrentPositionIndex) 1) 0)))
  (Transformation|SetRelativeRotation (Variables|Default|GetCurrentRotator) (Utilities|Array|Get(acopy) (Variables|Default|GetCurrentRotations) (Variables|Default|GetCurrentRotatorIndex)) true false) ; Smooth Movement = Sweep
  (if (and (and (Utilities|Operators|EqualEqual (Utilities|Array|Get(acopy) (Variables|Default|GetCurrentRotations)) (Utilities|Array|Get(acopy) (Variables|Default|GetRotationPoints) (Utilities|Array|Get(acopy) (Variables|Default|GetSolvedPositionIndex))) 5.0) (Utilities|Operators|EqualEqual (Utilities|Array|Get(acopy) (Variables|Default|GetCurrentRotations) 1) (Utilities|Array|Get(acopy) (Variables|Default|GetRotationPoints) (Utilities|Array|Get(acopy) (Variables|Default|GetSolvedPositionIndex) 1)) 5.0)) (Utilities|Operators|EqualEqual (Utilities|Array|Get(acopy) (Variables|Default|GetCurrentRotations) 2) (Utilities|Array|Get(acopy) (Variables|Default|GetRotationPoints) (Utilities|Array|Get(acopy) (Variables|Default|GetSolvedPositionIndex) 2)) 5.0))
    (Variables|Default|SetSolved true)
    (Class|BPIReact|React(Message) (Variables|Default|GetActorToReact) true)
    (goto _label Reset)
    (else
      (Variables|Default|GetSolved
        (:then
          (Variables|Default|SetSolved false)
          (Utilities|FlowControl|DoOnce true :!label _label
            (:Completed
              (Class|BPIReact|React(Message) (Variables|Default|GetActorToReact) false))))
        (:else)))))

(event Custom|Right
  (bind _rotationamount (Variables|Default|GetRotationAmount))
  (bind _currentrotations (Variables|Default|GetCurrentRotations))
  (bind _currentrotatorindex (Variables|Default|GetCurrentRotatorIndex))
  (bind _output (Utilities|Array|Get(acopy) _currentrotations _currentrotatorindex))
  (bind _returnvalue (Math|Rotator|CombineRotators _rotationamount _output))
  (Transformation|SetRelativeRotation (Variables|Default|GetCurrentRotator) _returnvalue false false)
  (Utilities|Array|SetArrayElem (Variables|Default|GetCurrentRotations) (Variables|Default|GetCurrentRotatorIndex) _returnvalue)
  (Variables|Default|SetCurrentPositionIndex (Math|Integer|SelectInt 0 (+ (Variables|Default|GetCurrentPositionIndex) 1) (> (+ (Variables|Default|GetCurrentPositionIndex) 1) (Utilities|Array|LastIndex (Variables|Default|GetRotationPoints)))))
  (Transformation|SetRelativeRotation (Variables|Default|GetCurrentRotator) (Utilities|Array|Get(acopy) (Variables|Default|GetCurrentRotations) (Variables|Default|GetCurrentRotatorIndex)) true false) ; Smooth Movement = Sweep
  (if (and (and (Utilities|Operators|EqualEqual (Utilities|Array|Get(acopy) (Variables|Default|GetCurrentRotations)) (Utilities|Array|Get(acopy) (Variables|Default|GetRotationPoints) (Utilities|Array|Get(acopy) (Variables|Default|GetSolvedPositionIndex))) 5.0) (Utilities|Operators|EqualEqual (Utilities|Array|Get(acopy) (Variables|Default|GetCurrentRotations) 1) (Utilities|Array|Get(acopy) (Variables|Default|GetRotationPoints) (Utilities|Array|Get(acopy) (Variables|Default|GetSolvedPositionIndex) 1)) 5.0)) (Utilities|Operators|EqualEqual (Utilities|Array|Get(acopy) (Variables|Default|GetCurrentRotations) 2) (Utilities|Array|Get(acopy) (Variables|Default|GetRotationPoints) (Utilities|Array|Get(acopy) (Variables|Default|GetSolvedPositionIndex) 2)) 5.0))
    (Variables|Default|SetSolved true)
    (Class|BPIReact|React(Message) (Variables|Default|GetActorToReact) true)
    (goto _label Reset)
    (else
      (Variables|Default|GetSolved
        (:then
          (Variables|Default|SetSolved false)
          (Utilities|FlowControl|DoOnce true :!label _label
            (:Completed
              (Class|BPIReact|React(Message) (Variables|Default|GetActorToReact) false))))
        (:else)))))

(event Custom|Up
  (bind _rotators (Variables|Default|GetRotators))
  (bind _returnvalue (Utilities|Array|LastIndex _rotators))
  (Utilities|IsValid (Variables|Default|GetCurrentRotator)
    (:Is%20Valid
      (Utilities|Array|SetArrayElem (Variables|Default|GetCurrentRotations) (Variables|Default|GetCurrentRotatorIndex) (Variables|/Script/Engine.SceneComponent|GetRelativeRotation (Variables|Default|GetCurrentRotator)))
      (if (> (+ (Variables|Default|GetCurrentRotatorIndex) 1) _returnvalue)
        (Variables|Default|SetCurrentRotator (Utilities|Array|Get(acopy) _rotators))
        (Variables|Default|SetCurrentRotatorIndex 0)
        (else
          (Variables|Default|SetCurrentRotator (Utilities|Array|Get(acopy) (Variables|Default|GetRotators) (Math|Integer|Clamp(Integer) (+ (Variables|Default|GetCurrentRotatorIndex) 1) 0 _returnvalue)))
          (Variables|Default|SetCurrentRotatorIndex (Math|Integer|Clamp(Integer) (+ (Variables|Default|GetCurrentRotatorIndex) 1) 0 _returnvalue)))))))

(event Input|EnhancedActionEvents|EnhancedInputActionIA_Interact
  (params (ActionValue :type Boolean) (ElapsedSeconds :type Float%20%28double-precision%29) (TriggeredSeconds :type Float%20%28double-precision%29) (InputAction :type Input%20Action%20Object%20Reference :default "/Game/Inputs/IA_Interact.IA_Interact"))
  (:Started
    (Class|CommonActivatableWidgetContainerBase|RemoveWidget (Utilities|ReturnMainStack (Game|GetPlayerController 0)) (Variables|Default|GetActiveWidget))
    (Utilities|FlowControl|DoOnce false :!label _label
      (:Completed
        (Utilities|SmoothPossess (Game|GetPlayerController 0) (Variables|Default|GetPlayerRef) 1.0)
        (Pawn|SetControlRotation (Game|GetPlayerController 0) (Variables|Default|GetControlRotation))
        (Math|Integer|DecrementInt (Variables|/Game/Blueprints/Core/BP_Player.BP_Player_C|GetCantMove (Variables|Default|GetPlayerRef))
          (:%20%20
            (goto _label Reset)))))))

(event Input|EnhancedActionEvents|EnhancedInputActionIA_Move
  (params (ActionValue :type Vector%202D%20Structure) (ElapsedSeconds :type Float%20%28double-precision%29) (TriggeredSeconds :type Float%20%28double-precision%29) (InputAction :type Input%20Action%20Object%20Reference :default "/Game/Inputs/IA_Move.IA_Move"))
  (bind (_x _y) (Math|Vector2D|BreakVector2D ActionValue))
  (:Started
    (if (> (Math|Float|Absolute(Float) _x) (Math|Float|Absolute(Float) _y)) ; True = left/right\nFalse = up/down
      (if (> _x 0.0)
        (CallFunction|Right)
        (else
          (CallFunction|Left)))
      (elif (> _y 0.0)
        (CallFunction|Up)
        (else
          (CallFunction|Down))))))

(event EventBeginPlay
  (bind _returnvalue (Math|Random|RandomInteger 10))
  (bind _rotators (Variables|Default|GetRotators))
  (bind _solvedpositionindex (Variables|Default|GetSolvedPositionIndex))
  (Utilities|Array|Clear _rotators)
  (Utilities|Array|Add _rotators (Variables|Default|GetR1Mesh))
  (Utilities|Array|Add _rotators (Variables|Default|GetR2Mesh))
  (Utilities|Array|Add _rotators (Variables|Default|GetR3Mesh))
  (Utilities|Array|Clear (Variables|Default|GetCurrentRotations))
  (Utilities|Array|Add (Variables|Default|GetCurrentRotations) (Variables|/Script/Engine.SceneComponent|GetRelativeRotation (Variables|Default|GetR1Mesh)))
  (Utilities|Array|Add (Variables|Default|GetCurrentRotations) (Variables|/Script/Engine.SceneComponent|GetRelativeRotation (Variables|Default|GetR2Mesh)))
  (Utilities|Array|Add (Variables|Default|GetCurrentRotations) (Variables|/Script/Engine.SceneComponent|GetRelativeRotation (Variables|Default|GetR3Mesh)))
  (Variables|Default|SetCurrentRotatorIndex 0)
  (Variables|Default|SetCurrentRotator (Utilities|Array|Get(acopy) (Variables|Default|GetRotators)))
  (Variables|Default|SetRotationAmount (Utilities|Array|Get(acopy) (Variables|Default|GetRotationPoints) 1))
  (Utilities|Array|Clear _solvedpositionindex)
  (Utilities|Array|Add _solvedpositionindex _returnvalue)
  (Utilities|Array|Add _solvedpositionindex _returnvalue)
  (Utilities|Array|Add _solvedpositionindex _returnvalue)
  (bind _outactors (Actor|GetAllActorsOfClass "/Game/Blueprints/World/BP_FinalHint.BP_FinalHint_C"))
  (Class|BPIFinalCode|GetCodeNumber(Message) _outactors (Variables|Default|GetSolvedPositionIndex)))

(event EventReact
  (params (Solved :type Boolean))
  (Variables|Default|SetIsInteractable true))

(event EventInteract
  (params (Sender :type Actor%20Object%20Reference))
  (bind _asbp_player (Utilities|Casting|CastToBP_Player Sender))
  (bind _output_get (Variables|Default|SetPlayerRef _asbp_player))
  (Math|Integer|IncrementInt (Variables|/Game/Blueprints/Core/BP_Player.BP_Player_C|GetCantMove _output_get)
    (:%20%20
      (Variables|Default|SetControlRotation (Pawn|GetControlRotation (Variables|Default|GetPlayerRef) :!class /Script/Engine.Pawn))
      (Utilities|SmoothPossess (Game|GetPlayerController 0) self 1.0)
      (bind _returnvalue (Class|CommonActivatableWidgetContainerBase|AddWidget (Utilities|ReturnMainStack (Game|GetPlayerController 0)) (Variables|Default|GetActivatableWidget)))
      (Variables|Default|SetActiveWidget _returnvalue))))

(fn ConstructionScript)

(fn ReturnInteractStatus
  (return (Variables|Default|GetIsInteractable)))

(fn ReturnSolvedStatus
  (return (Variables|Default|GetSolved)))
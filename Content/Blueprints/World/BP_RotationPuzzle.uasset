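; BP_RotationPuzzle is an interactable puzzle piece that steps through preset rotations, with one index counting as solved.
; Interact advances the wrapping index and sets RotationScene's relative rotation, which the construction script also previews.
; Reaching or leaving the solved index updates Solved and messages ActorToReact, with a DoOnce gating the unsolved message.
; React alternately enables and disables interaction, swapping mesh materials to match.
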(event EventReact
  (params (Solved :type Boolean))
  (Utilities|FlowControl|FlipFlop
    (:A
      (Rendering|Material|SetMaterial (Variables|Default|GetMesh) 0 (Variables|Default|GetActivationMaterial))
      (Rendering|Material|SetMaterial (Variables|Default|GetStaticMesh) 0 (Variables|Default|GetActivationMaterial))
      (Variables|Default|SetIsInteractable true))
    (:B
      (Rendering|Material|SetMaterial (Variables|Default|GetMesh) 0 "/Engine/EditorMeshes/ColorCalibrator/M_GreyBall.M_GreyBall")
      (Rendering|Material|SetMaterial (Variables|Default|GetStaticMesh) 0 "/Engine/EditorMeshes/ColorCalibrator/M_GreyBall.M_GreyBall")
      (Variables|Default|SetIsInteractable false))))

(event EventSetInteractStatus
  (params (IsInteractable :type Boolean))
  (Variables|Default|SetIsInteractable IsInteractable))

(event EventInteract
  (params (Sender :type Actor%20Object%20Reference))
  (Variables|Default|SetCurrentPositionIndex (Math|Integer|SelectInt 0 (+ (Variables|Default|GetCurrentPositionIndex) 1) (> (+ (Variables|Default|GetCurrentPositionIndex) 1) (Utilities|Array|LastIndex (Variables|Default|GetRotationPoints)))))
  (Transformation|SetRelativeRotation (Variables|Default|GetRotationScene) (Utilities|Array|Get(acopy) (Variables|Default|GetRotationPoints) (Variables|Default|GetCurrentPositionIndex)) true false) ; Smooth Movement = Sweep
  (if (== (Variables|Default|GetCurrentPositionIndex) (Variables|Default|GetSolvedPositionIndex))
    (Variables|Default|SetSolved true)
    (Class|BPIReact|React(Message) (Variables|Default|GetActorToReact) true)
    (goto _label Reset)
    (else
      (Variables|Default|GetSolved
        (:then
          (Variables|Default|SetSolved false)
          (Utilities|FlowControl|DoOnce true :!label _label
            (:Completed
              (Class|BPIReact|React(Message) (Variables|Default|GetActorToReact) false))))
        (:else)))))

(fn ConstructionScript
  (Transformation|SetRelativeRotation (Variables|Default|GetRotationScene) (Utilities|Array|Get(acopy) (Variables|Default|GetRotationPoints) (Variables|Default|GetCurrentPositionIndex)) false false))

(fn ReturnInteractStatus
  (return (Variables|Default|GetIsInteractable)))

(fn ReturnSolvedStatus
  (return (Variables|Default|GetSolved)))